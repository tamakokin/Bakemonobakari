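; Spline path actor that exposes position queries along its Spline component, likely for objects that travel the path.
; GetCurrentLocation converts a distance into a local-space point, with a Loop flag and a modulo wrap; as written, the wrap applies even when Loop is false.
; GetSplineLength returns the path length and IsArrived tests whether a distance has reached it.
; BeginPlay caches the actor location in BasePos.
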(event `self.ReceiveBeginPlay`
  (set `self.BasePos` (`self.K2_GetActorLocation`)))

(fn `Get Current Location`
  (params (Loop :type Boolean) (Length :type "Float (double-precision)"))
  (returns (Return :type "Vector Structure"))
  (if (not Loop)
    (set `self.LocalLength` Length))
  (set `self.LocalLength` (mod Length (`SplineComponent.GetSplineLength` (`self.Spline`))))
  (return (`SplineComponent.GetLocationAtDistanceAlongSpline` (`self.Spline`) (`self.LocalLength`) "Local")))

(fn `GetSplineLength`
  (returns (NewParam :type "Float (double-precision)"))
  (return (`SplineComponent.GetSplineLength` (`self.Spline`))))

(fn `IsArrived`
  (params (NewParam :type "Float (double-precision)"))
  (returns (NewParam1 :type Boolean))
  (return (>= NewParam (`SplineComponent.GetSplineLength` (`self.Spline`)))))

(fn `UserConstructionScript`)