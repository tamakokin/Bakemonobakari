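; Breakable vase prop that shatters when hit by the player's attack and drops a recovery item.
; An overlap on the Box from a "PlayerAttack"-tagged component, guarded by a one-shot Clash flag, applies damage and an impulse to the Vase04DM destructible mesh, plays a break sound and spawns RecoveryBP at an offset.
; Two seconds later it disables gravity and collision on the debris to save performance.
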(event `self.Box.OnComponentBeginOverlap`
  (params (OverlappedComponent :type "PrimitiveComponent Object Reference") (OtherActor :type "Actor Object Reference") (OtherComp :type "PrimitiveComponent Object Reference") (OtherBodyIndex :type Integer) (bFromSweep :type Boolean) (SweepResult :type "HitResult Structure (by ref)"))
  (bind _vase04_dm (`self.Vase04_DM`))
  (bind _vase04_dm_2 (`self.Vase04_DM`))
  (bind _returnvalue (`SceneComponent.K2_GetComponentLocation` _vase04_dm_2))
  ;[1 1 1] 攻撃を受けた際に破壊される（伴野）
  (if (and (`ActorComponent.ComponentHasTag` OtherComp "PlayerAttack") (not (`self.Clash`)))
    (`DestructibleComponent.ApplyDamage` _vase04_dm_2 10.0 _returnvalue (`KismetMathLibrary.MakeVector` -0.5 0.5 0.5) 500.0)
    (`GameplayStatics.PlaySoundAtLocation` "/Game/Sound/SE/VaseBreak.VaseBreak" _returnvalue (struct) 1.0 1.0 0.0 null null null)
    (set `self.Clash` true)
    ;[1 1 1] 回復アイテムを出す（松中）
    (`|SpawnActorFromClass` "/Game/Blueprints/RecoveryBP.RecoveryBP_C" (`KismetMathLibrary.MakeTransform` (+ (`self.K2_GetActorLocation`) (`self.OffsetLocation`))) "Undefined" "OverrideRootScale" null null)
    ;[1 1 1] 処理を軽くするため、一定時間経過後に重力とコリジョンを無効化（伴野）
    (`KismetSystemLibrary.Delay` 2.0)
    (`PrimitiveComponent.SetEnableGravity` _vase04_dm false)
    (`PrimitiveComponent.SetCollisionEnabled` _vase04_dm "NoCollision")))

(fn `UserConstructionScript`)