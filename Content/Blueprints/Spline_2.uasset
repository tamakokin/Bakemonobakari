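; Spline path actor that exposes distance-based queries along its Spline component.
; GetCurrentLocation returns a local-space point at a given distance, using modulo to wrap around the spline length when looping.
; GetSplineLength and IsArrived report the total length and whether a distance has reached the end.
; BeginPlay caches the actor's location in BasePos, which none of these functions read.
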(event `self.ReceiveBeginPlay`
  (set `self.BasePos` (`self.K2_GetActorLocation`)))

(fn `Get Current Location`
  (params (Loop :type Boolean) (Length :type "Float (double-precision)"))
  (returns (Return :type "Vector Structure"))
  (if Loop
    (set `self.LocalLength` (mod Length (`SplineComponent.GetSplineLength` (`self.Spline`))))
    (else
      (set `self.LocalLength` Length)))
  (return (`SplineComponent.GetLocationAtDistanceAlongSpline` (`self.Spline`) (`self.LocalLength`) "Local")))

(fn `GetSplineLength`
  (returns (NewParam :type "Float (double-precision)"))
  (return (`SplineComponent.GetSplineLength` (`self.Spline`))))

(fn `IsArrived`
  (params (NewParam :type "Float (double-precision)"))
  (returns (NewParam1 :type Boolean))
  (return (>= NewParam (`SplineComponent.GetSplineLength` (`self.Spline`)))))

(fn `UserConstructionScript`)