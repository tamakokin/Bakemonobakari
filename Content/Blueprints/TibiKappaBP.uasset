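; Blueprint for the TibiKappa enemy, which moves through components and triggers a hit stop around player attacks.
; BeginPlay passes its jump, straight and rotation components to ENEMYJUMPSTART and sets the time dilation values.
; When a PlayerAttack-tagged component stops overlapping the skeletal mesh, global time slows briefly, then resets after a short delay that is itself stretched by the dilation.
; The slowdown only starts when time is at normal speed, preventing stacking.
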(event `self.ReceiveBeginPlay`
  (bind _enemy_jump_start_ (`self.ENEMY_JUMP_START_`))
  (`ENEMY_JUMP_START_Component.SetJumpComponent` _enemy_jump_start_ (`self.ENEMY_TYPE_JUMP_`))
  (`ENEMY_JUMP_START_Component.SetStraightComponent` _enemy_jump_start_ (`self.ENEMY_TYPE_STRAIGHT_`))
  (`ENEMY_JUMP_START_Component.SetEnemyRoteComponent` _enemy_jump_start_ (`self.Enemy_Rote_`))
  (set `self.Dilation_0` 0.1)
  (set `self.ResetDilation_0` 1.0))

(event `self.SkeletalMesh.OnComponentEndOverlap`
  (params (OverlappedComponent :type "PrimitiveComponent Object Reference") (OtherActor :type "Actor Object Reference") (OtherComp :type "PrimitiveComponent Object Reference") (OtherBodyIndex :type Integer))
  (if (`ActorComponent.ComponentHasTag` OtherComp "PlayerAttack")
    (if (== (`GameplayStatics.GetGlobalTimeDilation`) (`self.ResetDilation_0`))
      (`GameplayStatics.SetGlobalTimeDilation` (`self.Dilation_0`))
      (`KismetSystemLibrary.Delay` 0.02)
      (`GameplayStatics.SetGlobalTimeDilation` (`self.ResetDilation_0`)))))

(fn `UserConstructionScript`
  (`parent.UserConstructionScript`))