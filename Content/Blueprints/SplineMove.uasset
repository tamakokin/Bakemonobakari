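; Actor that travels along a spline at a set speed, toggling a breaking flag on a House as it moves.
; Each Tick advances distance along the spline, sweeps the actor to that point offset by the spline's base position, and faces the skeletal mesh along the movement.
; A CheckInScreen test on the start position's Y and Z zeroes speed and distance and clears the flag when it fails.
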(event `self.ReceiveBeginPlay`
  (set `self.StartPos` (`self.K2_GetActorLocation`))
  (set `/Game/Blueprints/House.IsBreak` false (`self.House`)))

(event `self.ReceiveTick`
  (params (DeltaSeconds :type "Float (single-precision)"))
  (bind _speed (`self.Speed`))
  ;[1 1 1] 現在の座標を取得
  (bind _return (`/Game/Blueprints/Spline.Get Current Location` (`self.spline`) false (`self.distance`)))
  (set `self.OldPos` (+ _return (`/Game/Blueprints/Spline.BasePos` (`self.spline`))))
  ;[1 1 1] スピードが0なら移動しない
  (if (< 0.0 _speed)
    (bind _output_get (set `self.distance` (+ (`self.distance`) (* DeltaSeconds _speed))))
    (bind _return_2 (`/Game/Blueprints/Spline.Get Current Location` (`self.spline`) false _output_get))
    (bind _returnvalue (+ _return_2 (`/Game/Blueprints/Spline.BasePos` (`self.spline`))))
    (`self.K2_SetActorLocation` _returnvalue true)
    (`SceneComponent.K2_SetRelativeRotation` (`self.SkeletalMesh`) (`KismetMathLibrary.Conv_VectorToRotator` (- _returnvalue (`self.OldPos`))) false false)
    (set `/Game/Blueprints/House.IsBreak` true (`self.House`))
    (bind _returnvalue_2 (`CheckInScreen.Check` (`self.CheckInScreen`) (`KismetMathLibrary.Conv_Vector4ToVector` (`KismetMathLibrary.MakeVector4` 0.0 (.y (`self.StartPos`)) (.z (`self.StartPos`))))))
    (if (not _returnvalue_2)
      (set `self.Speed` 0.0)
      (set `self.distance` 0.0)
      (set `/Game/Blueprints/House.IsBreak` false (`self.House`)))))

(fn `UserConstructionScript`)