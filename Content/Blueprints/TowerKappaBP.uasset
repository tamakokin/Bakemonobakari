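; Boss-fight actor for a tower of up to seven kappas that loses one segment per player hit.
; CreateEvent trims the stack to three or five segments in the first two BossPhase values.
; Capsule overlaps tagged PlayerAttack only set the IsDamage flag; nothing here calls DamageEvent.
; DamageEvent decrements TowerHP, destroys that index's capsule and mesh, then clears IsInvincible and IsDamage after a short delay.
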(event `self.ReceiveBeginPlay`)

(event `self.CreateEvent`
  ;[1 1 1] フェースによって、異なる個数を作る（陳7/19）
  (switch `int` (`self._BossPhase`)
    (:`0`
      (`ActorComponent.K2_DestroyComponent` (`self.SkeletalMesh4`))
      (`ActorComponent.K2_DestroyComponent` (`self.SkeletalMesh5`))
      (`ActorComponent.K2_DestroyComponent` (`self.SkeletalMesh6`))
      (`ActorComponent.K2_DestroyComponent` (`self.SkeletalMesh7`))
      (`ActorComponent.K2_DestroyComponent` (`self.Capsule5`))
      (`ActorComponent.K2_DestroyComponent` (`self.Capsule4`))
      (`ActorComponent.K2_DestroyComponent` (`self.Capsule6`))
      (`ActorComponent.K2_DestroyComponent` (`self.Capsule7`)))
    (:`1`
      (`ActorComponent.K2_DestroyComponent` (`self.SkeletalMesh6`))
      (`ActorComponent.K2_DestroyComponent` (`self.SkeletalMesh7`))
      (`ActorComponent.K2_DestroyComponent` (`self.Capsule6`))
      (`ActorComponent.K2_DestroyComponent` (`self.Capsule7`)))))

(event `self.DestroyEvent`
  ;[1 1 1] 削除処理（陳7/19）
  (`self.K2_DestroyActor`))

(event `self.DamageEvent`
  ;[1 1 1] プレイヤーの攻撃を受けたら、個数を減らす（陳7/19）
  (bind _output_get (set `self._TowerHP` (- (`self._TowerHP`) 1)))
  (switch `int` _output_get
    (:`0`
      (`ActorComponent.K2_DestroyComponent` (`self.Capsule1`))
      (`ActorComponent.K2_DestroyComponent` (`self.SkeletalMesh1`)))
    (:`1`
      (`ActorComponent.K2_DestroyComponent` (`self.Capsule2`))
      (`ActorComponent.K2_DestroyComponent` (`self.SkeletalMesh2`)))
    (:`2`
      (`ActorComponent.K2_DestroyComponent` (`self.Capsule3`))
      (`ActorComponent.K2_DestroyComponent` (`self.SkeletalMesh3`)))
    (:`3`
      (`ActorComponent.K2_DestroyComponent` (`self.Capsule4`))
      (`ActorComponent.K2_DestroyComponent` (`self.SkeletalMesh4`)))
    (:`4`
      (`ActorComponent.K2_DestroyComponent` (`self.Capsule5`))
      (`ActorComponent.K2_DestroyComponent` (`self.SkeletalMesh5`)))
    (:`5`
      (`ActorComponent.K2_DestroyComponent` (`self.Capsule6`))
      (`ActorComponent.K2_DestroyComponent` (`self.SkeletalMesh6`)))
    (:`6`
      (`ActorComponent.K2_DestroyComponent` (`self.Capsule7`))
      (`ActorComponent.K2_DestroyComponent` (`self.SkeletalMesh7`))))
  (`KismetSystemLibrary.Delay` 0.3)
  (set `self._IsInvincible` false)
  (set `self._IsDamage` false))

(event `self.Capsule1.OnComponentBeginOverlap`
  (params (OverlappedComponent :type "PrimitiveComponent Object Reference") (OtherActor :type "Actor Object Reference") (OtherComp :type "PrimitiveComponent Object Reference") (OtherBodyIndex :type Integer) (bFromSweep :type Boolean) (SweepResult :type "HitResult Structure (by ref)"))
  ;[1 1 1] プレイヤーの攻撃を受ける処理（陳7/19）
  (if (`ActorComponent.ComponentHasTag` OtherComp "PlayerAttack")
    (if (not (`self._IsDamage`)) :!label _label
      (set `self._IsDamage` true))))

(event `self.Capsule2.OnComponentBeginOverlap`
  (params (OverlappedComponent :type "PrimitiveComponent Object Reference") (OtherActor :type "Actor Object Reference") (OtherComp :type "PrimitiveComponent Object Reference") (OtherBodyIndex :type Integer) (bFromSweep :type Boolean) (SweepResult :type "HitResult Structure (by ref)"))
  ;[1 1 1] プレイヤーの攻撃を受ける処理（陳7/19）
  (if (`ActorComponent.ComponentHasTag` OtherComp "PlayerAttack")
    (goto _label)))

(event `self.Capsule3.OnComponentBeginOverlap`
  (params (OverlappedComponent :type "PrimitiveComponent Object Reference") (OtherActor :type "Actor Object Reference") (OtherComp :type "PrimitiveComponent Object Reference") (OtherBodyIndex :type Integer) (bFromSweep :type Boolean) (SweepResult :type "HitResult Structure (by ref)"))
  ;[1 1 1] プレイヤーの攻撃を受ける処理（陳7/19）
  (if (`ActorComponent.ComponentHasTag` OtherComp "PlayerAttack")
    (goto _label)))

(event `self.Capsule4.OnComponentBeginOverlap`
  (params (OverlappedComponent :type "PrimitiveComponent Object Reference") (OtherActor :type "Actor Object Reference") (OtherComp :type "PrimitiveComponent Object Reference") (OtherBodyIndex :type Integer) (bFromSweep :type Boolean) (SweepResult :type "HitResult Structure (by ref)"))
  ;[1 1 1] プレイヤーの攻撃を受ける処理（陳7/19）
  (if (`ActorComponent.ComponentHasTag` OtherComp "PlayerAttack")
    (goto _label)))

(event `self.Capsule5.OnComponentBeginOverlap`
  (params (OverlappedComponent :type "PrimitiveComponent Object Reference") (OtherActor :type "Actor Object Reference") (OtherComp :type "PrimitiveComponent Object Reference") (OtherBodyIndex :type Integer) (bFromSweep :type Boolean) (SweepResult :type "HitResult Structure (by ref)"))
  ;[1 1 1] プレイヤーの攻撃を受ける処理（陳7/19）
  (if (`ActorComponent.ComponentHasTag` OtherComp "PlayerAttack")
    (goto _label)))

(event `self.Capsule6.OnComponentBeginOverlap`
  (params (OverlappedComponent :type "PrimitiveComponent Object Reference") (OtherActor :type "Actor Object Reference") (OtherComp :type "PrimitiveComponent Object Reference") (OtherBodyIndex :type Integer) (bFromSweep :type Boolean) (SweepResult :type "HitResult Structure (by ref)"))
  ;[1 1 1] プレイヤーの攻撃を受ける処理（陳7/19）
  (if (`ActorComponent.ComponentHasTag` OtherComp "PlayerAttack")
    (goto _label)))

(event `self.Capsule7.OnComponentBeginOverlap`
  (params (OverlappedComponent :type "PrimitiveComponent Object Reference") (OtherActor :type "Actor Object Reference") (OtherComp :type "PrimitiveComponent Object Reference") (OtherBodyIndex :type Integer) (bFromSweep :type Boolean) (SweepResult :type "HitResult Structure (by ref)"))
  ;[1 1 1] プレイヤーの攻撃を受ける処理（陳7/19）
  (if (`ActorComponent.ComponentHasTag` OtherComp "PlayerAttack")
    (goto _label)))

(fn `UserConstructionScript`)