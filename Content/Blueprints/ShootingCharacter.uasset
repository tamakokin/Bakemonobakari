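; Player character for an auto-running shooting stage, apparently Stage 3, that jumps, crouches and fires bullets.
; Tick pushes it along +X until death, at half input while damaged, and caches the anim Blueprint whose in-air state gates jump and crouch.
; Attack spawns a PlayerBullet ahead of the player and sets IsAttack, which nothing here clears.
; The logic that sets IsCrouch is disconnected, and the facing-rotation function is never called here.
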(event `self.ReceiveBeginPlay`)

(event `InputAction|Jump`
  (params (Key :type "Key Structure"))
  ;[1 1 1] ジャンプ処理（7/29）
  (:`Pressed`
    (if (`self.IsDead`)
      _
      (elif (not (`/Game/Models/PlayerCharacter/Animation/Player_Stage3AnimBP.IsInAir?` (stale `self.ReceiveTick` _asplayer_stage_3anim_bp)))
        (`self.Jump`))))
  (:`Released`
    (`self.StopJumping`)))

(event `self.ReceiveTick`
  (params (DeltaSeconds :type "Float (single-precision)"))
  (if (`self.IsDead`)
    _
    (elif (`self.IsDamage`)
      (`self.AddMovementInput` (0.5 0.0 0.0))
      (else
        (`self.AddMovementInput` (1.0 0.0 0.0)))))
  (bind _asplayer_stage_3anim_bp (cast `/Game/Models/PlayerCharacter/Animation/Player_Stage3AnimBP` (`SkeletalMeshComponent.GetAnimInstance` (`self.Mesh`))))
  (if (`/Game/Models/PlayerCharacter/Animation/Player_Stage3AnimBP.IsInAir?` _asplayer_stage_3anim_bp)
    _
    (elif (`self.IsDead`)
      _
      (elif (`self.IsCrouch`)
        (`self.Crouch`)))))

(event `InputAction|Attack`
  (params (Key :type "Key Structure"))
  ;[1 1 1] 攻撃処理（7/29）
  (:`Pressed`
    (if (not (`self.IsAttack`))
      (set `self.IsAttack` true)
      (`KismetSystemLibrary.PrintString` "attack")
      (`|SpawnActorFromClass` "/Game/Blueprints/PlayerBullet.PlayerBullet_C" (`KismetMathLibrary.MakeTransform` (+ (`self.K2_GetActorLocation` (`GameplayStatics.GetPlayerCharacter` 0)) (50.0 0.0 0.0))) "Undefined" "OverrideRootScale" null null))))

(event `InputAction|Crouch`
  (params (Key :type "Key Structure"))
  ;[1 1 1] しゃがみ処理（7/29）
  (:`Released`
    (`self.UnCrouch`)
    (set `self.IsCrouch` false)))

(fn `SetPlayerRotation`
  (bind _mesh (`self.Mesh`))
  (if (== (.y (`MovementComponent.Velocity` (`self.CharacterMovement`))) 0.0)
    (`SceneComponent.K2_SetRelativeRotation` :`self` _mesh)
    (elif (`self.IsFaceRight`)
      (`SceneComponent.K2_SetRelativeRotation` _mesh (struct :`Yaw` 90.0) false false)
      (else
        (`SceneComponent.K2_SetRelativeRotation` _mesh (struct :`Yaw` -90.0) false false))))
  (return))

(fn `UserConstructionScript`)