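; Spotlight Blueprint that makes its light flicker by setting a new random intensity every Tick.
; It averages ten uniform random draws to approximate a bell curve, mirrors results in the upper half back down from Max, and snaps those below Threshold to Min for occasional dropouts.
; The random expression is re-rolled for each branch test and the final assignment, so the tested value differs from the applied one.
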(event `self.ReceiveBeginPlay`
  ;[1 1 1] BeginPlay
  ;;[1 1 1] 変数の初期化
  (set `self.max` 20.0)
  (set `self.min` 0.0)
  (set `self.threshold` 4.0))

(event `self.ReceiveTick`
  (params (DeltaSeconds :type "Float (single-precision)"))
  (bind _max (`self.max`))
  (bind _min (`self.min`))
  (bind _returnvalue (/ (+ (+ (+ (+ (+ (+ (+ (+ (+ (`KismetMathLibrary.RandomFloatInRange` _min _max) (`KismetMathLibrary.RandomFloatInRange` _min _max)) (`KismetMathLibrary.RandomFloatInRange` _min _max)) (`KismetMathLibrary.RandomFloatInRange` _min _max)) (`KismetMathLibrary.RandomFloatInRange` _min _max)) (`KismetMathLibrary.RandomFloatInRange` _min _max)) (`KismetMathLibrary.RandomFloatInRange` _min _max)) (`KismetMathLibrary.RandomFloatInRange` _min _max)) (`KismetMathLibrary.RandomFloatInRange` _min _max)) (`KismetMathLibrary.RandomFloatInRange` _min _max)) 10.0))
  (bind _returnvalue_2 (`KismetMathLibrary.Abs` (- _returnvalue (`self.max`))))
  ;[1 1 1] Tick
  ;;[1 1 1] 値の補正
  (if (> _returnvalue (/ (`self.max`) 2.0))
    (if (< _returnvalue_2 (`self.threshold`))
      ;;[1 1 1] Intensityに代入
      (`LightComponent.SetIntensity` (`self.SpotLightComponent`) (`self.min`))
      (else
        (`LightComponent.SetIntensity` (`self.SpotLightComponent`) _returnvalue_2)))
    (elif (< _returnvalue (`self.threshold`))
      (`LightComponent.SetIntensity` (`self.SpotLightComponent`) (`self.min`))
      (else
        (`LightComponent.SetIntensity` (`self.SpotLightComponent`) _returnvalue)))))

(fn `UserConstructionScript`)