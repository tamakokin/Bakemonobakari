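; Blueprint for the Hitodama enemy, providing hit feedback and show/hide handling; no movement logic appears here.
; Hit spawns an offset cut particle and applies a brief hit-stop by dipping global time dilation.
; Destroy and Ind hide and restore the enemy by toggling mesh visibility and capsule/mesh collision instead of destroying the actor.
; HitEfect spawns Enemy_EffectBP while visible; the PlayerAttack end-overlap check triggers nothing.
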(event `self.ReceiveBeginPlay`
  (set `self.Dilation` 0.1)
  (set `self.ResetDilation` 1.0))

(event `self.Hit`
  (`GameplayStatics.SpawnEmitterAtLocation` "/Game/Effects/Hit_Cut.Hit_Cut" (`KismetMathLibrary.MakeVector` (+ (.x (`self.K2_GetActorLocation`)) 50.0) (.y (`self.K2_GetActorLocation`)) (.z (`self.K2_GetActorLocation`))) (struct) (2.0 2.0 2.0))
  ;[1 1 1] HitStop
  (if (== (`GameplayStatics.GetGlobalTimeDilation`) (`self.ResetDilation`))
    (`GameplayStatics.SetGlobalTimeDilation` (`self.Dilation`))
    (`KismetSystemLibrary.Delay` 0.022)
    (`GameplayStatics.SetGlobalTimeDilation` (`self.ResetDilation`))))

(event `self.SkeletalMesh.OnComponentEndOverlap`
  (params (OverlappedComponent :type "PrimitiveComponent Object Reference") (OtherActor :type "Actor Object Reference") (OtherComp :type "PrimitiveComponent Object Reference") (OtherBodyIndex :type Integer))
  ;[1 1 1] HitStop
  (if (`SceneComponent.bVisible` (`self.SkeletalMesh`))
    (if (`ActorComponent.ComponentHasTag` OtherComp "PlayerAttack")
      _)))

(fn `Destroy`
  (bind _m_penemymesh (`self.m_pEnemyMesh`))
  (bind _m_penemymesh_2 (`self.m_pEnemyMesh`))
  (`/Engine/EditorBlueprintResources/StandardMacros.IsValid` (`self.m_pCapsuleComp`)
    (:`Is Valid`
      (`/Engine/EditorBlueprintResources/StandardMacros.IsValid` _m_penemymesh_2
        (:`Is Valid`
          (if (`SceneComponent.bVisible` _m_penemymesh_2)
            (`PrimitiveComponent.SetCollisionEnabled` (`self.m_pCapsuleComp`) "NoCollision")
            (`SceneComponent.SetVisibility` _m_penemymesh false false)
            (`PrimitiveComponent.SetCollisionEnabled` _m_penemymesh "NoCollision")))))))

(fn `Hit Efect`
  (if (`SceneComponent.bVisible` (`self.SkeletalMesh`))
    (`|SpawnActorFromClass` "/Game/Effects/Enemy_EffectBP.Enemy_EffectBP_C" (`self.GetTransform`) "Undefined" "OverrideRootScale" null null)))

(fn `Ind`
  (bind _m_penemymesh (`self.m_pEnemyMesh`))
  (`/Engine/EditorBlueprintResources/StandardMacros.IsValid` (`self.m_pCapsuleComp`)
    (:`Is Valid`
      (`/Engine/EditorBlueprintResources/StandardMacros.IsValid` (`self.m_pEnemyMesh`)
        (:`Is Valid`
          (if (not (`SceneComponent.bVisible` (`self.m_pEnemyMesh`)))
            (`PrimitiveComponent.SetCollisionEnabled` (`self.m_pCapsuleComp`) "QueryAndPhysics")
            (`SceneComponent.SetVisibility` _m_penemymesh true false)
            (`PrimitiveComponent.SetCollisionEnabled` _m_penemymesh "QueryAndPhysics")))))))

(fn `UserConstructionScript`)