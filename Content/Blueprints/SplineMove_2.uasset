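; Actor Blueprint that moves itself continuously along a looping path supplied by its Spline reference.
; Each Tick, while Speed is positive, it advances Distance by Speed times delta time and queries the spline's custom GetCurrentLocation with looping enabled.
; It adds the spline's BasePos to that point and teleports there without sweeping, leaving rotation untouched.
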(event `self.ReceiveTick`
  (params (DeltaSeconds :type "Float (single-precision)"))
  (bind _speed (`self.Speed`))
  (bind _distance (`self.distance`))
  (if (< 0.0 _speed)
    (set `self.distance` (+ _distance (* DeltaSeconds _speed)))
    (bind _return (`/Game/Blueprints/Spline_2.Get Current Location` (`self.spline`) true _distance))
    (`self.K2_SetActorLocation` (+ (`KismetMathLibrary.MakeVector` (.x _return) (.y _return) (.z _return)) (`/Game/Blueprints/Spline_2.BasePos` (`self.spline`))) false true)))

(fn `UserConstructionScript`)