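; Bakemono enemy Blueprint that handles hit feedback and toggles the enemy between active and disabled states.
; Hit spawns particles and applies a brief hit-stop through global time dilation, skipped if time is already dilated.
; Destroy disables capsule and mesh collision and calls MeshOff, while Ind restores visibility and collision, so the actor is never actually destroyed.
; HitEfect plays an offset particle and crash sound; the PlayerAttack end-overlap check does nothing.
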(event `self.ReceiveBeginPlay`
  (set `self.Dilation` 0.1)
  (set `self.ResetDilation` 1.0))

(event `self.Hit`
  (`GameplayStatics.SpawnEmitterAtLocation` "/Game/Effects/Hit/Hit.Hit" (`self.K2_GetActorLocation`))
  ;[1 1 1] HitStop
  (if (== (`GameplayStatics.GetGlobalTimeDilation`) (`self.ResetDilation`))
    (`GameplayStatics.SetGlobalTimeDilation` (`self.Dilation`))
    (`KismetSystemLibrary.Delay` 0.022)
    (`GameplayStatics.SetGlobalTimeDilation` (`self.ResetDilation`))))

(event `self.SkeletalMesh.OnComponentEndOverlap`
  (params (OverlappedComponent :type "PrimitiveComponent Object Reference") (OtherActor :type "Actor Object Reference") (OtherComp :type "PrimitiveComponent Object Reference") (OtherBodyIndex :type Integer))
  ;[1 1 1] HitStop
  (if (`SceneComponent.bVisible` (`self.SkeletalMesh`))
    (if (`ActorComponent.ComponentHasTag` OtherComp "PlayerAttack")
      _)))

(fn `Destroy`
  (bind _m_penemymesh (`self.m_pEnemyMesh`))
  (`/Engine/EditorBlueprintResources/StandardMacros.IsValid` (`self.m_pCapsuleComp`)
    (:`Is Valid`
      (`/Engine/EditorBlueprintResources/StandardMacros.IsValid` _m_penemymesh
        (:`Is Valid`
          (if (`SceneComponent.bVisible` _m_penemymesh)
            (`PrimitiveComponent.SetCollisionEnabled` (`self.m_pCapsuleComp`) "NoCollision")
            (`self.MeshOff`)
            (`PrimitiveComponent.SetCollisionEnabled` (`self.m_pEnemyMesh`) "NoCollision")))))))

(fn `Hit Efect`
  (params (EfectPos :type "Vector Structure"))
  (if (not (`self.bHidden`))
    (`GameplayStatics.SpawnEmitterAtLocation` "/Game/Effects/Enemy_GoHome/Enemy_GoHome.Enemy_GoHome" (+ EfectPos (`self.K2_GetActorLocation`)))
    (`GameplayStatics.PlaySound2D` "/Game/Sound/SE/crash.crash" 1.0 1.0 0.0 null null)))

(fn `Ind`
  (bind _m_penemymesh (`self.m_pEnemyMesh`))
  (`/Engine/EditorBlueprintResources/StandardMacros.IsValid` (`self.m_pCapsuleComp`)
    (:`Is Valid`
      (`/Engine/EditorBlueprintResources/StandardMacros.IsValid` (`self.m_pEnemyMesh`)
        (:`Is Valid`
          (if (not (`SceneComponent.bVisible` (`self.m_pEnemyMesh`)))
            (`PrimitiveComponent.SetCollisionEnabled` (`self.m_pCapsuleComp`) "QueryAndPhysics")
            (`SceneComponent.SetVisibility` _m_penemymesh true false)
            (`PrimitiveComponent.SetCollisionEnabled` _m_penemymesh "QueryAndPhysics")))))))

(fn `UserConstructionScript`)