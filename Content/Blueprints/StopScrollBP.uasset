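; StopScrollBP is a scroll-lock trigger that holds the camera at a point until its enemy count is cleared.
; The first overlap passes a DoOnce before the PlayerCharacter tag check, then points CameraControl at CameraPosActor.
; DecrementEnemyCount, not called within this Blueprint, lowers EnemyCount and returns the camera to the player when it reaches zero.
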(event `self.ReceiveActorBeginOverlap`
  (params (OtherActor :type "Actor Object Reference"))
  (`/Engine/EditorBlueprintResources/StandardMacros.DoOnce` false
    (:`Completed`
      (if (`self.ActorHasTag` OtherActor "PlayerCharacter")
        (`CameraControl.SetTargetActor` (`self.CameraControl`) (`self.CameraPosActor`) 100.0)))))

(fn `DecrementEnemyCount`
  (if (> (`self.EnemyCount`) 0)
    (bind _result (`/Engine/EditorBlueprintResources/StandardMacros.DecrementInt` (`self.EnemyCount`))
      (:`  `
        (set `self.EnemyCount` _result)
        (if (<= (`self.EnemyCount`) 0)
          (`CameraControl.SetTargetPlayerActor` (`self.CameraControl`)))))))

(fn `UserConstructionScript`)