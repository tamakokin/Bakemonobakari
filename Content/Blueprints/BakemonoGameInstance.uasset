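; Game instance for Bakemono that swaps streamed levels behind a loading screen widget.
; LoadingScreenStart stores the current and next level names, shows the widget and passes LoadLevel as the fade-in callback.
; LoadLevel unloads the current level unless it is Stage_Origin, streams in the next without blocking, then flags the widget as finished.
; LoadingScreenEnd fades the widget out and removes it through the FadeOutEnd callback.
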(event `LoadingScreenStart`
  (params (NextLevel :type Name) (CurrentLevel :type Name))
  ;[1 1 1] ローディング画面処理（陳7/12）
  (set `self.NextLevel` NextLevel)
  (set `self.CurrentLevel` CurrentLevel)
  ;;[1 1 1] ローディング画面生成
  (bind _returnvalue (`|CreateWidget` "/Game/UI/LoadingScreenWidget.LoadingScreenWidget_C" (`GameplayStatics.GetPlayerController` 0)))
  (bind _output_get (set `self.LoadingScreen` _returnvalue))
  (`UserWidget.AddToViewport` _output_get 100)
  ;;[1 1 1] ローディング画面フェードイン
  (`/Game/UI/LoadingScreenWidget.FadeInFunction` (`self.LoadingScreen`) (delegate `LoadLevel`)))

(event `LoadLevel`
  (bind _loadingscreen (`self.LoadingScreen`))
  ;[1 1 1] ローディング画面処理（陳7/12）
  ;;[1 1 1] フェードイン終了してからステージをローディング
  (if (!= (`self.CurrentLevel`) "Stage_Origin")
    (`GameplayStatics.UnloadStreamLevel` (`self.CurrentLevel`)))
  (`GameplayStatics.LoadStreamLevel` (`self.NextLevel`) true)
  (set `/Game/UI/LoadingScreenWidget.IsLoadFinished` true _loadingscreen)
  (`/Game/UI/LoadingScreenWidget.LoadFinish` _loadingscreen))

(event `LoadingScreenEnd`
  ;[1 1 1] ローディング画面処理（陳7/12）
  ;;[1 1 1] ローディング終了してフェードアウト
  (`/Game/UI/LoadingScreenWidget.FadeOutFunction` (`self.LoadingScreen`) (delegate `FadeOutEnd`)))

(event `FadeOutEnd`
  ;[1 1 1] ローディング画面処理（陳7/12）
  ;;[1 1 1] ローディング終了してフェードアウト
  (`Widget.RemoveFromParent` (`self.LoadingScreen`)))