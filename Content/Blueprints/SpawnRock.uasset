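; SpawnRock is a spawner actor that periodically creates Rock actors at its own location.
; Tick increments a frame counter and, every 200 ticks, passes the spawner's location to CheckInScreen, so the interval depends on frame rate.
; When that check returns false, presumably meaning off screen, it spawns a Rock and copies its own Force value onto it.
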(event `self.ReceiveTick`
  (params (DeltaSeconds :type "Float (single-precision)"))
  (bind _output_get (set `self.Count` (+ (`self.Count`) 1)))
  (if (== (mod _output_get 200) 0)
    (bind _returnvalue (`CheckInScreen.Check` (`self.CheckInScreen`) (`self.K2_GetActorLocation`)))
    (if (not _returnvalue)
      (bind _returnvalue_2 (`|SpawnActorFromClass` "/Game/Blueprints/Rock.Rock_C" (`KismetMathLibrary.Conv_VectorToTransform` (`self.K2_GetActorLocation`)) "Undefined" "OverrideRootScale" null null))
      (set `/Game/Blueprints/Rock.Force` (`self.Force`) _returnvalue_2))))

(fn `UserConstructionScript`)