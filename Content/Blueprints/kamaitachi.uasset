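; Kamaitachi enemy Blueprint that senses what lies ahead and exposes attack, hit effect and hide/restore functions.
; Tick line-traces a short way along world +Y or -Y according to yaw, passing player and ground tag results to ENEMYCHOPSTART.
; BeginAttack and EndAttack toggle the Box collision, and HitEfect spawns an effect actor.
; Destroy only hides the mesh and disables collision, so Ind can restore both.
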(event `self.ReceiveTick`
  (params (DeltaSeconds :type "Float (single-precision)"))
  (bind _returnvalue (`self.K2_GetActorLocation`))
  (bind _enemy_chop_start_ (`self.ENEMY_CHOP_START_`))
  (bind _enemy_chop_start__2 (`self.ENEMY_CHOP_START_`))
  (if (< 89.0 (.yaw (`self.K2_GetActorRotation`)))
    (bind (_outhit _returnvalue_2) (`KismetSystemLibrary.LineTraceSingle` _returnvalue (+ _returnvalue (0.0 100.0 0.0)) "TraceTypeQuery1"))
    (if _returnvalue_2
      (bind (_bblockinghit _binitialoverlap _time _distance _location _impactpoint _normal _impactnormal _physmat _hitactor) (`GameplayStatics.BreakHitResult` _outhit))
      (`ENEMY_CHOP_START_Component.SetHitPlayer` _enemy_chop_start__2 (`self.ActorHasTag` _hitactor "PlayerCharacter"))
      (`ENEMY_CHOP_START_Component.SetHitGround` _enemy_chop_start__2 (`self.ActorHasTag` _hitactor "Ground")))
    (else
      (bind (_outhit_2 _returnvalue_3) (`KismetSystemLibrary.LineTraceSingle` _returnvalue (+ _returnvalue (0.0 -100.0 0.0)) "TraceTypeQuery1"))
      (if _returnvalue_3
        (bind (_bblockinghit_2 _binitialoverlap_2 _time_2 _distance_2 _location_2 _impactpoint_2 _normal_2 _impactnormal_2 _physmat_2 _hitactor_2) (`GameplayStatics.BreakHitResult` _outhit_2))
        (`ENEMY_CHOP_START_Component.SetHitPlayer` _enemy_chop_start_ (`self.ActorHasTag` _hitactor_2 "PlayerCharacter"))
        (`ENEMY_CHOP_START_Component.SetHitGround` _enemy_chop_start_ (`self.ActorHasTag` _hitactor_2 "Ground"))))))

(fn `BeginAttack`
  (`PrimitiveComponent.SetCollisionEnabled` (`self.Box`) "QueryAndPhysics"))

(fn `Destroy`
  (bind _m_penemymesh (`self.m_pEnemyMesh`))
  (bind _m_penemymesh_2 (`self.m_pEnemyMesh`))
  (`/Engine/EditorBlueprintResources/StandardMacros.IsValid` (`self.m_pCapsuleComp`)
    (:`Is Valid`
      (`/Engine/EditorBlueprintResources/StandardMacros.IsValid` _m_penemymesh_2
        (:`Is Valid`
          (if (`SceneComponent.bVisible` _m_penemymesh_2)
            (`PrimitiveComponent.SetCollisionEnabled` (`self.m_pCapsuleComp`) "NoCollision")
            (`SceneComponent.SetVisibility` _m_penemymesh false false)
            (`PrimitiveComponent.SetCollisionEnabled` _m_penemymesh "NoCollision")
            (`self.EndAttack`)))))))

(fn `EndAttack`
  (`PrimitiveComponent.SetCollisionEnabled` (`self.Box`) "NoCollision"))

(fn `Hit Efect`
  (if (`SceneComponent.bVisible` (`self.SkeletalMesh`))
    (`|SpawnActorFromClass` "/Game/Effects/Enemy_EffectBP.Enemy_EffectBP_C" (`self.GetTransform`) "Undefined" "OverrideRootScale" null null)))

(fn `Ind`
  (bind _m_penemymesh (`self.m_pEnemyMesh`))
  (`/Engine/EditorBlueprintResources/StandardMacros.IsValid` (`self.m_pCapsuleComp`)
    (:`Is Valid`
      (`/Engine/EditorBlueprintResources/StandardMacros.IsValid` (`self.m_pEnemyMesh`)
        (:`Is Valid`
          (if (not (`SceneComponent.bVisible` (`self.m_pEnemyMesh`)))
            (`PrimitiveComponent.SetCollisionEnabled` (`self.m_pCapsuleComp`) "QueryAndPhysics")
            (`SceneComponent.SetVisibility` _m_penemymesh true false)
            (`PrimitiveComponent.SetCollisionEnabled` _m_penemymesh "QueryAndPhysics")))))))

(fn `UserConstructionScript`)