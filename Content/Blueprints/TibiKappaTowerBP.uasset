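; TibiKappaTowerBP is a Blueprint with a skeletal mesh that adds a brief hit-stop effect around player attacks.
; When a component tagged PlayerAttack ends overlap with the mesh, it switches global time dilation to a set value, then restores it after a very short delay.
; The effect starts only if time dilation is at its reset value, so hit-stops do not stack.
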(event `self.SkeletalMesh.OnComponentEndOverlap`
  (params (OverlappedComponent :type "PrimitiveComponent Object Reference") (OtherActor :type "Actor Object Reference") (OtherComp :type "PrimitiveComponent Object Reference") (OtherBodyIndex :type Integer))
  (if (`ActorComponent.ComponentHasTag` OtherComp "PlayerAttack")
    (if (== (`GameplayStatics.GetGlobalTimeDilation`) (`self.ResetDilation_0`))
      (`GameplayStatics.SetGlobalTimeDilation` (`self.Dilation_0`))
      (`KismetSystemLibrary.Delay` 0.02)
      (`GameplayStatics.SetGlobalTimeDilation` (`self.ResetDilation_0`)))))

(fn `UserConstructionScript`
  (`parent.UserConstructionScript`))