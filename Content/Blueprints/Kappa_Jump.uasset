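; Kappa_Jump is an enemy Blueprint that handles hiding, restoring and damage effects for a Kappa enemy, with no jump logic in its own graph.
; Des_1 hides the enemy mesh and disables mesh and capsule collision, leaving the actor alive instead of destroying it.
; Indication_1 restores visibility and query-and-physics collision if the mesh is hidden.
; EnemyDamageEvent_1 spawns Enemy_EffectBP at the actor's transform.
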(event `Des_1`
  (bind _m_penemymesh (`self.m_pEnemyMesh`))
  (`/Engine/EditorBlueprintResources/StandardMacros.IsValid` (`self.m_pCapsuleComp`)
    (:`Is Valid`
      (`/Engine/EditorBlueprintResources/StandardMacros.IsValid` (`self.m_pEnemyMesh`)
        (:`Is Valid`
          (`PrimitiveComponent.SetCollisionEnabled` (`self.m_pCapsuleComp`) "NoCollision")
          (`SceneComponent.SetVisibility` _m_penemymesh false false)
          (`PrimitiveComponent.SetCollisionEnabled` _m_penemymesh "NoCollision"))))))

(event `EnemyDamageEvent_1`
  (`|SpawnActorFromClass` "/Game/Effects/Enemy_EffectBP.Enemy_EffectBP_C" (`self.GetTransform`) "Undefined" "OverrideRootScale" null null))

(event `Indication_1`
  (bind _m_penemymesh (`self.m_pEnemyMesh`))
  (`/Engine/EditorBlueprintResources/StandardMacros.IsValid` (`self.m_pCapsuleComp`)
    (:`Is Valid`
      (`/Engine/EditorBlueprintResources/StandardMacros.IsValid` (`self.m_pEnemyMesh`)
        (:`Is Valid`
          (if (not (`SceneComponent.bVisible` (`self.m_pEnemyMesh`)))
            (`PrimitiveComponent.SetCollisionEnabled` (`self.m_pCapsuleComp`) "QueryAndPhysics")
            (`SceneComponent.SetVisibility` _m_penemymesh true false)
            (`PrimitiveComponent.SetCollisionEnabled` _m_penemymesh "QueryAndPhysics")))))))

(fn `UserConstructionScript`)