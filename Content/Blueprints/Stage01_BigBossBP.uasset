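; Stage 01 big boss that fights through three attack phases separated by player knockbacks, then dies.
; Tick drives a phase enum, spawning timed waves of small bosses and Shirikodama plus a phase-scaled kappa tower, gated by DoAttack and DoOnce.
; Overlaps from Enemy-tagged actors or PlayerAttack components advance the phase.
; Knockback phases lerp the player to a set point before advancing.
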(event `self.ReceiveBeginPlay`
  (set `self.DoAttack` true)
  (`KismetSystemLibrary.Delay` (`self.NormalAttackFaseDelayTime`))
  (set `self.DoAttack` false))

(event `self.ReceiveTick`
  (params (DeltaSeconds :type "Float (single-precision)"))
  (`KismetSystemLibrary.PrintString` (`|GetEnumeratorNameAsString` (`self.EFase`)) true true (struct :`G` 0.66 :`B` 1.0 :`A` 1.0) 0.0)
  (switch `/Game/Enums/EStage01BossFase` (`self.EFase`)
    (:`NewEnumerator0`
      (`self.NormalAttackFase`)
      (`self.SpawnTower` 1))
    (:`NewEnumerator3`
      (`self.NockbackFase` :!label _label))
    (:`NewEnumerator1`
      (`self.NormalAttackFase`)
      (`self.SpawnTower` 2))
    (:`NewEnumerator4`
      (goto _label))
    (:`NewEnumerator2`
      (`self.FinalAttackFase`)
      (`self.SpawnTower` 3))
    (:`NewEnumerator5`
      (`self.Boss_Die`)
      (`self.K2_DestroyActor`))))

(event `self.SkeletalMesh.OnComponentBeginOverlap`
  (params (OverlappedComponent :type "PrimitiveComponent Object Reference") (OtherActor :type "Actor Object Reference") (OtherComp :type "PrimitiveComponent Object Reference") (OtherBodyIndex :type Integer) (bFromSweep :type Boolean) (SweepResult :type "HitResult Structure (by ref)"))
  (if (or (`self.ActorHasTag` OtherActor "Enemy") (`ActorComponent.ComponentHasTag` OtherComp "PlayerAttack"))
    (set `self.EFase` (cast `/Game/Enums/EStage01BossFase` (+ (`self.EFase`) 1)))))

(fn `UserConstructionScript`)