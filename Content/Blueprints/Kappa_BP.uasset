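; Kappa_BP is a kappa enemy Blueprint that handles its hit effect, hiding and removal.
; EnemyDamageEvent spawns an Enemy_EffectBP at the actor's transform.
; Des disables capsule collision and hides the enemy mesh without destroying the actor.
; When destroyed, it decrements the enemy count on a valid StopScroll reference.
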(event `self.ReceiveDestroyed`
  (bind _stopscroll (`self.StopScroll`))
  (`/Engine/EditorBlueprintResources/StandardMacros.IsValid` _stopscroll
    (:`Is Valid`
      (`/Game/Blueprints/StopScrollBP.DecrementEnemyCount` _stopscroll))))

(event `self.Des`
  (`PrimitiveComponent.SetCollisionEnabled` (`self.m_pCapsuleComp`) "NoCollision")
  (`SceneComponent.SetVisibility` (`self.m_pEnemyMesh`) false false))

(event `self.EnemyDamageEvent`
  (`|SpawnActorFromClass` "/Game/Effects/Enemy_EffectBP.Enemy_EffectBP_C" (`self.GetTransform`) "Undefined" "OverrideRootScale" null null))

(fn `UserConstructionScript`)