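; Ladder actor Blueprint whose collision volumes scale with a LadderLength variable.
; The Construction Script places CollisionUpper just above the ladder's top and centers BoxCollision at half height, both offset along local Y.
; It sizes BoxCollision's vertical extent to fall short of the full length at both ends.
; The event graph holds only disabled placeholder events, so this file contains no climbing logic.
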(fn `UserConstructionScript`
  (locals (Ladder_Polygon :type Boolean) (ladder_Index :type Boolean))
  (bind _ladderlength (`self.ladderLength`))
  (bind _boxcollision (`self.BoxCollision`))
  (`SceneComponent.K2_SetRelativeLocation` (`self.CollisionUpper`) (`KismetMathLibrary.MakeVector` 0.0 20.0 (+ _ladderlength 1.0)) false true)
  (`SceneComponent.K2_SetRelativeLocation` _boxcollision (`KismetMathLibrary.MakeVector` 0.0 30.0 (/ _ladderlength 2.0)) false false)
  (`BoxComponent.SetBoxExtent` _boxcollision (`KismetMathLibrary.MakeVector` 20.0 5.0 (/ (- _ladderlength 80.0) 2.0)) true))