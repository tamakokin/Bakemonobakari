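; Okuriinu enemy Blueprint that can be hidden and shown again in place.
; Des disables capsule collision and hides the enemy mesh, while Indication restores both if the mesh is hidden.
; EnemyDamageEvent spawns an Enemy_EffectBP at the actor's transform.
; Destroyed is empty, and the logic that decrements the StopScroll enemy count is disconnected, so it never runs.
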(event `self.ReceiveDestroyed`)

(event `self.Des`
  (`PrimitiveComponent.SetCollisionEnabled` (`self.m_pCapsuleComp`) "NoCollision")
  (`SceneComponent.SetVisibility` (`self.m_pEnemyMesh`) false false))

(event `self.EnemyDamageEvent`
  (`|SpawnActorFromClass` "/Game/Effects/Enemy_EffectBP.Enemy_EffectBP_C" (`self.GetTransform`) "Undefined" "OverrideRootScale" null null))

(event `self.Indication`
  (if (not (`SceneComponent.bVisible` (`self.m_pEnemyMesh`)))
    (`PrimitiveComponent.SetCollisionEnabled` (`self.m_pCapsuleComp`) "QueryAndPhysics")
    (`SceneComponent.SetVisibility` (`self.m_pEnemyMesh`) true false)))

(fn `UserConstructionScript`)