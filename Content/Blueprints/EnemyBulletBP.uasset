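; Enemy bullet actor that flies along the world Y axis and destroys itself off screen or on touching a Player-tagged actor.
; Each Tick, CheckInScreen gates a fixed per-frame step, not scaled by delta time: +Y at zero yaw, -Y at negative yaw, none at positive yaw.
; The accumulated DeltaTime and the delayed DoOnce flag do not affect movement, and the overlap applies no damage here.
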(event `self.ReceiveBeginPlay`
  (set `self.DeltaTime` 0.0)
  (set `self.moveSpeedY` 12.0)
  (set `self.do once` true))

(event `self.ReceiveTick`
  (params (DeltaSeconds :type "Float (single-precision)"))
  (bind _yaw (.yaw (`SceneComponent.K2_GetComponentRotation` (`self.DefaultSceneRoot`))))
  (set `self.DeltaTime` (+ (`self.DeltaTime`) (`GameplayStatics.GetWorldDeltaSeconds`)))
  (bind _returnvalue (`CheckInScreen.Check` (`self.CheckInScreen`) (`self.K2_GetActorLocation`)))
  (if _returnvalue
    (if (`self.do once`)
      (`/Engine/EditorBlueprintResources/StandardMacros.DoOnce` false
        (:`Completed`
          (`KismetSystemLibrary.Delay` 0.4)
          (set `self.do once` false))))
    (if (== _yaw 0.0)
      (`self.K2_SetActorLocation` (`KismetMathLibrary.MakeVector` (.x (`self.K2_GetActorLocation`)) (+ (.y (`self.K2_GetActorLocation`)) (`self.moveSpeedY`)) (.z (`self.K2_GetActorLocation`))))
      (elif (< _yaw 0.0)
        (`self.K2_SetActorLocation` (`KismetMathLibrary.MakeVector` (.x (`self.K2_GetActorLocation`)) (- (.y (`self.K2_GetActorLocation`)) (`self.moveSpeedY`)) (.z (`self.K2_GetActorLocation`))))))
    (else
      (`self.K2_DestroyActor`))))

(event `self.ReceiveActorBeginOverlap`
  (params (OtherActor :type "Actor Object Reference"))
  (if (`self.ActorHasTag` OtherActor "Player")
    (`self.K2_DestroyActor`)))

(fn `UserConstructionScript`)